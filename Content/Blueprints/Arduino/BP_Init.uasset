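; BP_Init is a test Blueprint that links the game to an Arduino over a serial COM port.
; BeginPlay opens a hard-coded port, stores the connection and flushes it, and EndPlay closes it.
; Releasing R reads a string from the Arduino on demand and prints it, with on-screen messages reporting connection status and read failures.
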(event EventBeginPlay
  (bind (_bopened _returnvalue) (Class|Serial|OpenComPort 5 9600))
  (if _bopened
    (bind _output_get (Variables|Default|SetArduino _returnvalue))
    (Development|PrintString "Arduino Initialized")
    (Class|Serial|Flush _output_get)
    (else
      (Development|PrintString "Port not opened"))))

(event EventEndPlay
  (params (EndPlayReason :type EEndPlayReason%20Enum :default "Destroyed"))
  (bind _arduino (Variables|Default|GetArduino))
  (Utilities|IsValid _arduino
    (:Is%20Valid
      (Class|Serial|Close _arduino))))

(event Input|KeyboardEvents|R
  (params (Key :type Key%20Structure :default "None"))
  (bind _arduino (Variables|Default|GetArduino))
  (:Released
    (Development|PrintString "R is pressed")
    (Utilities|IsValid _arduino
      (:Is%20Valid
        (bind (_bsuccess _returnvalue) (Class|Serial|ReadString _arduino))
        (if _bsuccess
          (Development|PrintString _returnvalue)
          (else
            (Development|PrintString "Error Reading String")))))))

(fn ConstructionScript)