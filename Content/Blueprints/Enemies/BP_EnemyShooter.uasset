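; BP_EnemyShooter is an enemy that turns to face the player and fires projectiles when its PawnSensing component sees the first-person character.
; Each sighting snaps the actor's rotation toward the player.
; When allowed, it spawns a PlayerAttack actor at ShootPoint and launches it forward with a velocity-change impulse on its mesh.
; A CanShoot flag and a short Delay throttle the firing rate.
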(event OnSeePawn(PawnSensing)
  (params (Pawn :type Pawn%20Object%20Reference))
  (bind _asfirst_person_character (Utilities|Casting|CastToFirstPersonCharacter Pawn))
  (Utilities|FlowControl|Sequence
    (:then_0
      (Transformation|SetActorRotation (Math|Rotator|FindLookatRotation (Transformation|GetActorLocation) (Transformation|GetActorLocation _asfirst_person_character))))
    (:then_1
      (if (Variables|Default|GetcanShoot)
        (bind _returnvalue (Game|SpawnActorfromClass "/Game/FirstPersonCPP/Blueprints/PlayerAttack.PlayerAttack_C" (Transformation|GetWorldTransform (Variables|Default|GetShootPoint)) "Undefined" 0 0))
        (Physics|AddImpulse (Variables|/Game/FirstPersonCPP/Blueprints/PlayerAttack.PlayerAttack_C|GetStaticMesh1 _returnvalue) (* (Math|Vector|GetForwardVector (Variables|Default|GetShootPoint)) 2e+02) "None" true)
        (Variables|Default|SetcanShoot false)
        (Utilities|FlowControl|Delay 2.0)
        (Variables|Default|SetcanShoot true)))))

(fn ConstructionScript)