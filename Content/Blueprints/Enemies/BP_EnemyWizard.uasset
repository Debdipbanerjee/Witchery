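; BP_EnemyWizard is an enemy that teleports between three preset points and shoots fireballs at the player.
; A looping Disapper/Appear cycle drives two timelines that animate the shared MPC_E_Dissolve parameter, moving the wizard to a random checkpoint while dissolved.
; PawnSensing turns it toward the seen player and calls ShootAttack, gated by a cooldown and the Hidden flag, to spawn and launch a fireball.
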(event OnSeePawn(PawnSensing)
  (params (Pawn :type Pawn%20Object%20Reference))
  ;[1 1 1] AI
  (bind _asfirst_person_character (Utilities|Casting|CastToFirstPersonCharacter Pawn))
  (Utilities|FlowControl|Sequence
    (:then_0
      (Transformation|SetActorRotation (Math|Rotator|FindLookatRotation (Transformation|GetActorLocation) (Transformation|GetActorLocation _asfirst_person_character))))
    (:then_1
      (if (and (Variables|Default|GetcanShoot) (not (Variables|Default|Gethidden)))
        (Utilities|FlowControl|Sequence
          (:then_0
            (CallFunction|ShootAttack))
          (:then_1
            (Utilities|FlowControl|Delay 5.0)
            (Variables|Default|SetcanShoot true)))))))

(event Custom|Disapper
  ;[1 1 1] Disapper
  (Development|PrintString "Disappearing")
  (Variables|Default|Sethidden true)
  (bind _dissolve (Timeline|Timeline_3 PlayFromStart)
    (:Update
      (Rendering|Material|SetScalarParameterValue "/Game/WitcherySimulator/Material/MPC_E_Dissolve.MPC_E_Dissolve" "Dissolve" _dissolve :!class /Script/Engine.KismetMaterialLibrary))
    (:Finished
      (Utilities|FlowControl|Delay 0.1)
      (CallFunction|Appear))))

(event Custom|Appear
  (bind _checkpoints (Variables|Default|GetCheckpoints))
  ;[1 1 1] Re-Appearing
  (Development|PrintString "appearing")
  (bind _output_get (Variables|Default|SetTargetPos (Utilities|Array|Get(acopy) _checkpoints (Math|Random|RandomInteger (Utilities|Array|Length _checkpoints)))))
  (Transformation|SetActorLocation _output_get false false)
  (bind _gather (Timeline|Timeline_0 PlayFromStart)
    (:Update
      (Rendering|Material|SetScalarParameterValue "/Game/WitcherySimulator/Material/MPC_E_Dissolve.MPC_E_Dissolve" "Dissolve" _gather :!class /Script/Engine.KismetMaterialLibrary))
    (:Finished
      (Variables|Default|Sethidden false)
      (Utilities|FlowControl|Delay 5.0)
      (CallFunction|Disapper))))

(event EventBeginPlay
  ;[1 1 1] Setting Respawn Points
  (Variables|Default|SetCheckpoints (Utilities|Array|MakeArray (Transformation|GetWorldLocation (Variables|Default|GetSceneTransform1)) (Transformation|GetWorldLocation (Variables|Default|GetSceneTransform2)) (Transformation|GetWorldLocation (Variables|Default|GetSceneTransform3))))
  (Utilities|FlowControl|Delay 5.0)
  (CallFunction|Disapper))

(fn ConstructionScript)

(fn ShootAttack
  (bind _returnvalue (Game|SpawnActorfromClass "/Game/FirstPersonCPP/Blueprints/BP_E_Fireball.BP_E_Fireball_C" (Transformation|GetWorldTransform (Variables|Default|GetShootPoint)) "Undefined" 0 0))
  (Physics|AddImpulse (Variables|/Game/FirstPersonCPP/Blueprints/BP_E_Fireball.BP_E_Fireball_C|GetTrail _returnvalue) (* (Math|Vector|GetForwardVector (Variables|Default|GetShootPoint)) 1e+01) "None" false)
  (Variables|Default|SetcanShoot false))