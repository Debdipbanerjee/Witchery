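; BP_Enemy_Teleport is a test actor that previews an enemy teleport effect, triggered once by E or set on a nine-second loop by 2.
; EnemyTeleport activates the Teleport Niagara system, then two chained timelines drive Dissolve and Gather in the MPC_E_Dissolve parameter collection.
; When they finish, it deactivates the effect and resets both parameters after a delay.
; Nodes binding From and To skeletal meshes to Niagara are unconnected, and no actor movement occurs.
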(event Custom|EnemyTeleport
  ;[3 0.5 0] Enemy Teleport Blueprint
  (Components|Activation|Activate (Variables|Default|GetTeleport) true)
  (Utilities|FlowControl|Delay 0.3)
  (bind _dissolve (Timeline|TeleportStart PlayFromStart)
    (:Update
      (Rendering|Material|SetScalarParameterValue "/Game/WitcherySimulator/Material/MPC_E_Dissolve.MPC_E_Dissolve" "Dissolve" _dissolve :!class /Script/Engine.KismetMaterialLibrary))
    (:Finished
      (bind _gather (Timeline|TeleportEnd PlayFromStart)
        (:Update
          (Rendering|Material|SetScalarParameterValue "/Game/WitcherySimulator/Material/MPC_E_Dissolve.MPC_E_Dissolve" "Gather" _gather :!class /Script/Engine.KismetMaterialLibrary))
        (:Finished
          (Components|Activation|Deactivate (Variables|Default|GetTeleport))
          ;[1 0 0] Test
          (Utilities|FlowControl|Delay 2.0)
          (Rendering|Material|SetScalarParameterValue "/Game/WitcherySimulator/Material/MPC_E_Dissolve.MPC_E_Dissolve" "Dissolve" 0.95 :!class /Script/Engine.KismetMaterialLibrary)
          (Rendering|Material|SetScalarParameterValue "/Game/WitcherySimulator/Material/MPC_E_Dissolve.MPC_E_Dissolve" "Gather" -0.2 :!class /Script/Engine.KismetMaterialLibrary))))))

(event EventBeginPlay)

(event Collision|EventActorBeginOverlap
  (params (OtherActor :type Actor%20Object%20Reference)))

(event EventTick
  (params (DeltaSeconds :type Float%20%28single-precision%29)))

(event Input|KeyboardEvents|2
  (params (Key :type Key%20Structure :default "None"))
  (:Pressed
    (Utilities|Time|SetTimerbyEvent (delegate Custom|EnemyTeleport) 9.0 true)))

(event Input|KeyboardEvents|E
  (params (Key :type Key%20Structure :default "None"))
  (:Pressed
    (CallFunction|EnemyTeleport)))

(fn ConstructionScript)